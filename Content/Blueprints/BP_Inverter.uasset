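; BP_Inverter is a logic actor that acts as a NOT gate on the signal of its ActivationSource.
; On BeginPlay it waits a tick, fires Activated if the source starts inactive, then binds to the source's Activated and Deactivated events to emit the opposite.
; GetValue returns the negated active state and one minus the source's activation value, supporting both boolean and analog signals.
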(event `self.ReceiveBeginPlay`
  (bind _activation_source (`self.Activation Source`))
  (bind _activation_source_2 (`self.Activation Source`))
  (`KismetSystemLibrary.DelayUntilNextTick`)
  (`/Engine/EditorBlueprintResources/StandardMacros.IsValid` _activation_source_2
    (:`Is Valid`
      (bind _isactive (`self.GetValue` _activation_source_2))
      (if (not _isactive)
        (set `self.Outputting Signal` true)
        (`self.Activated`)))
    (:`Is Not Valid`
      _))
  (`parent.ReceiveBeginPlay`)
  (`/Engine/EditorBlueprintResources/StandardMacros.IsValid` _activation_source
    (:`Is Valid`
      (add `self.Activated` _activation_source (delegate `InverterActivated`))
      (add `self.Deactivated` _activation_source (delegate `InverterDeactivated`)))))

(event `InverterActivated`
  (set `self.Outputting Signal` false)
  (`self.Deactivated`))

(event `InverterDeactivated`
  (set `self.Outputting Signal` true)
  (`self.Activated`))

(fn `GetValue`
  (returns (IsActive :type Boolean) (ActivationValue :type "Float (double-precision)"))
  (bind (_isactive _activationvalue) (`self.GetValue` (`self.Activation Source`)))
  (return (not _isactive) (- 1.0 _activationvalue)))

(fn `UserConstructionScript`
  (`parent.UserConstructionScript`))