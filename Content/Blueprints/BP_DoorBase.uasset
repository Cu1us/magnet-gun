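; BP_DoorBase is a base door Blueprint driven by an ActivationSource, warning on BeginPlay if that is invalid.
; In dynamic mode, Tick maps the source's activation value through a curve into SetOpenAmount; otherwise activate and deactivate events play or reverse the DoorSlide timeline.
; When a TriggerBox overlap ends, it reapplies the desired amount if the actual one differs.
; SetOpenAmount is empty here, so this class contains no door movement itself.
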(event `self.ReceiveTick`
  (params (DeltaSeconds :type "Float (single-precision)"))
  (bind _activationsource (`self.ActivationSource`))
  (if (`self.Dynamic Open`)
    (`/Engine/EditorBlueprintResources/StandardMacros.IsValid` _activationsource
      (:`Is Valid`
        (bind (_isactive _activationvalue) (`/Game/Blueprints/BP_Activator.GetValue` _activationsource))
        (`self.SetOpenAmount` (`KismetMathLibrary.GetRuntimeFloatCurveValue` (`self.Dynamic Open Curve`) _activationvalue))))))

(event `self.ReceiveBeginPlay`
  (bind _activationsource (`self.ActivationSource`))
  (`/Engine/EditorBlueprintResources/StandardMacros.IsValid` _activationsource
    (:`Is Valid`
      (if (not (`self.Dynamic Open`))
        (add `/Game/Blueprints/BP_Activator.Activated` _activationsource (delegate `Open`))
        (add `/Game/Blueprints/BP_Activator.Deactivated` _activationsource (delegate `Close`))))
    (:`Is Not Valid`
      (`KismetSystemLibrary.PrintString` "Door was spawned without valid activation source!" true true (struct :`R` 1.0 :`G` 0.020499 :`A` 1.0) 5.0))))

(event `Open`
  (bind (_direction _opendistance) (`Timeline|DoorSlide` :!label _label)
    (:`Update`
      (`self.SetOpenAmount` _opendistance))))

(event `Close`
  (goto _label :!via `Reverse`))

(event `self.TriggerBox.OnComponentEndOverlap`
  (params (OverlappedComponent :type "PrimitiveComponent Object Reference") (OtherActor :type "Actor Object Reference") (OtherComp :type "PrimitiveComponent Object Reference") (OtherBodyIndex :type Integer))
  (bind _desired_open_amount (`self.Desired Open Amount`))
  (if (!= (`self.Actual Open Amount`) _desired_open_amount)
    (`self.SetOpenAmount` _desired_open_amount)))

(fn `SetOpenAmount`
  (params (`OpenAmount (0-1)` :type "Float (double-precision)")))

(fn `UserConstructionScript`)