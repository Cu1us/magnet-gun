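; BP_SignalSplitter is a signal node that, despite its name, acts as an AND gate, activating only while both its left and right activators are active.
; Any input change re-evaluates both sides, playing or reversing timelines that fade left, right and top visibility on a dynamic material.
; It fires Activated or Deactivated only when the combined state changes.
; GetValue returns that state with the clamped average of both input values.
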(event `self.ReceiveBeginPlay`
  (bind _activatorleft (`self.ActivatorLeft`))
  (bind _activatorright (`self.ActivatorRight`))
  (`|ExecutionSequence`
    (:`then_0`
      (`/Engine/EditorBlueprintResources/StandardMacros.IsValid` (`self.DynamicMaterial`)
        (:`Is Not Valid`
          (bind _returnvalue (`KismetMaterialLibrary.CreateDynamicMaterialInstance` "/Game/Materials/M_SignalSplitter.M_SignalSplitter"))
          (bind _output_get (set `self.DynamicMaterial` _returnvalue))
          (`PrimitiveComponent.SetMaterial` (`self.SignalSplitter`) 0 _output_get))))
    (:`then_1`
      (`/Engine/EditorBlueprintResources/StandardMacros.IsValid` _activatorleft
        (:`Is Valid`
          (add `self.Activated` _activatorleft (delegate `ActivateLeft`))
          (add `self.Deactivated` _activatorleft (delegate `DeactivateLeft`)))
        (:`Is Not Valid`
          (`KismetSystemLibrary.PrintString` "Signal splitter has no Left Activator" true true (struct :`R` 1.0 :`A` 1.0))))
      (`/Engine/EditorBlueprintResources/StandardMacros.IsValid` _activatorright
        (:`Is Valid`
          (add `self.Activated` _activatorright (delegate `ActivateRight`))
          (add `self.Deactivated` _activatorright (delegate `DeactivateRight`)))
        (:`Is Not Valid`
          (`KismetSystemLibrary.PrintString` "Signal splitter has no Right Activator" true true (struct :`R` 1.0 :`A` 1.0)))))))

(event `ActivateLeft`
  (bind _dynamicmaterial (`self.DynamicMaterial`))
  (bind _isactive (`self.GetValue` (`self.ActivatorLeft`) :!label _label))
  (bind _isactive_2 (`self.GetValue` (`self.ActivatorRight`)))
  (`|ExecutionSequence`
    (:`then_0`
      (if _isactive_2
        (bind (_direction _visibility) (`Timeline|RightVisTimeline` :!label _label_2)
          (:`Update`
            (`MaterialInstanceDynamic.SetScalarParameterValue` _dynamicmaterial "RightVisibility" _visibility)))
        (else
          (goto _label_2 :!via `Reverse`))))
    (:`then_1`
      (if _isactive
        (bind (_direction_2 _visibility_2) (`Timeline|LeftVisTimeline` :!label _label_3)
          (:`Update`
            (`MaterialInstanceDynamic.SetScalarParameterValue` _dynamicmaterial "LeftVisibility" _visibility_2)))
        (else
          (goto _label_3 :!via `Reverse`))))
    (:`then_2`
      (bind _returnvalue (and _isactive_2 _isactive))
      (if _returnvalue
        (bind (_direction_3 _visibility_3) (`Timeline|TopVisTimeline` :!label _label_4)
          (:`Update`
            (`MaterialInstanceDynamic.SetScalarParameterValue` _dynamicmaterial "TopVisibility" _visibility_3)))
        (else
          (goto _label_4 :!via `Reverse`))))
    (:`then_3`
      (if (xor _returnvalue (`self.SignalPropagated`))
        (bind _output_get (set `self.SignalPropagated` _returnvalue))
        (if _output_get
          (`self.Activated`)
          (else
            (`self.Deactivated`)))))))

(event `ActivateRight`
  (goto _label))

(event `DeactivateLeft`
  (goto _label))

(event `DeactivateRight`
  (goto _label))

(fn `GetValue`
  (returns (IsActive :type Boolean) (ActivationValue :type "Float (double-precision)"))
  (`|ExecutionSequence`
    (:`then_0`
      (bind (_isactive _activationvalue) (`self.GetValue` (`self.ActivatorLeft`))))
    (:`then_1`
      (bind (_isactive_2 _activationvalue_2) (`self.GetValue` (`self.ActivatorRight`))))
    (:`then_2`
      (return (`self.SignalPropagated`) (`KismetMathLibrary.FClamp` (/ (+ _activationvalue _activationvalue_2) 2.0))))))

(fn `UserConstructionScript`)