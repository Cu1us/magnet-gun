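; BP_MagnetBall is a physics ball that can be colored, aimed at a surface point and launched toward it.
; SetBeamTarget stores the point and normal, switching between main and seek beams and updating the ball material and a spawned target decal.
; While launching, Tick drives velocity toward the point offset by the ball's radius, easing off within the last meter via clamped squared distance.
; Enable and Disable control the visuals and halt any launch.
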(event `On Destroyed` :!signature `self.OnDestroyed`
  (params (DestroyedActor :type "Actor Object Reference"))
  ; Begin Play
  ;; On Destroyed
  (`self.K2_DestroyActor` (`self.TargetDecal`)))

(event `self.ReceiveBeginPlay`
  ; Begin Play
  (`|ExecutionSequence`
    (:`then_0`
      (add `self.OnDestroyed` (delegate `On Destroyed`))
      (bind _returnvalue (`|SpawnActorFromClass` "/Game/Blueprints/BP_TargetDecal.BP_TargetDecal_C" (`self.GetTransform`) "AlwaysSpawn" "MultiplyWithRoot" null null))
      (set `self.TargetDecal` _returnvalue))
    (:`then_1`
      (`/Engine/EditorBlueprintResources/StandardMacros.IsValid` (`self.BallMaterial`)
        (:`Is Not Valid`
          (`self.SetupMaterial`))))))

(event `self.ReceiveTick`
  (params (DeltaSeconds :type "Float (single-precision)"))
  (if (`self.Is Launching`)
    (`PrimitiveComponent.SetPhysicsLinearVelocity` (`self.Ball`) (* (`self.Get Launch Dir`) (`self.LaunchVelocity`) (`KismetMathLibrary.FClamp` (`KismetMathLibrary.Vector_DistanceSquared` (/ (`self.Get Launch Target`) 100.0) (/ (`SceneComponent.K2_GetComponentLocation` (`self.Ball`)) 100.0)))) false "None")))

(event `Enable`
  (params (Color :type "LinearColor Structure"))
  (bind _ballmaterial (`self.BallMaterial`))
  (`|ExecutionSequence`
    (:`then_0`
      (`MaterialInstanceDynamic.SetVectorParameterValue` _ballmaterial "PatternColor" Color)
      (`MaterialInstanceDynamic.SetScalarParameterValue` _ballmaterial "PatternVisible" 1.0))
    (:`then_1`
      (`NiagaraComponent.SetVariableLinearColor` (`self.BeamMain`) "Beam Color" Color))
    (:`then_2`
      (`/Game/Blueprints/BP_TargetDecal.Set Color` (`self.TargetDecal`) Color))
    (:`then_3`
      (`self.Unlaunch`))))

(event `Disable`
  (`MaterialInstanceDynamic.SetScalarParameterValue` (`self.BallMaterial`) "PatternVisible" 0.0)
  (`SceneComponent.SetVisibility` (`self.BeamMain`) false false)
  (`SceneComponent.SetVisibility` (`Actor.RootComponent` (`self.TargetDecal`)) false false)
  (`SceneComponent.SetVisibility` (`self.BeamSeek`) false false)
  (`self.Unlaunch`))

(event `Set Beam Target`
  (params (InValue :type "Vector Structure") (`Beam Hit Normal` :type "Vector Structure") (`Is Valid Target` :type Boolean))
  (bind _beamseek (`self.BeamSeek`))
  (bind _targetdecal (`self.TargetDecal`))
  (bind _ballmaterial (`self.BallMaterial`))
  (bind _beammain (`self.BeamMain`))
  (set `self.TargetLocation` InValue)
  (set `self.TargetNormal` `Beam Hit Normal`)
  (`MaterialInstanceDynamic.SetVectorParameterValue` _ballmaterial "BeamTargetWorld" (`KismetMathLibrary.Conv_VectorToLinearColor` InValue))
  (`MaterialInstanceDynamic.SetScalarParameterValue` _ballmaterial "ValidTarget" (select `bool` `Is Valid Target` :`true` 1.0 :!type "Float (single-precision)"))
  (if `Is Valid Target`
    (`NiagaraComponent.SetVariablePosition` _beammain "Beam End" InValue)
    (`SceneComponent.SetVisibility` _beammain true false)
    (`SceneComponent.SetVisibility` (`Actor.RootComponent` _targetdecal) true false)
    (`SceneComponent.SetVisibility` (`self.BeamSeek`) false false)
    (`/Game/Blueprints/BP_TargetDecal.Point From Pos` _targetdecal InValue `Beam Hit Normal` true)
    (else
      (`NiagaraComponent.SetVariablePosition` _beamseek "Beam End" InValue)
      (`SceneComponent.SetVisibility` _beamseek true false)
      (`SceneComponent.SetVisibility` (`Actor.RootComponent` (`self.TargetDecal`)) true false)
      (`SceneComponent.SetVisibility` (`self.BeamMain`) false false)
      (`/Game/Blueprints/BP_TargetDecal.Point From Pos` (`self.TargetDecal`) InValue `Beam Hit Normal` false))))

(fn `Launch`
  (set `self.Is Launching` true)
  (`PrimitiveComponent.SetPhysicsLinearVelocity` (`self.Ball`) (* (`self.Get Launch Dir`) (`self.LaunchVelocity`)) false "None"))

(fn `ToggleLaunch`
  (returns (`New Launching Status` :type Boolean))
  (if (`self.Is Launching`)
    (`self.Unlaunch`)
    (return false)
    (else
      (`self.Launch`)
      (return true))))

(fn `Unlaunch`
  (set `self.Is Launching` false)
  (`PrimitiveComponent.SetPhysicsLinearVelocity` (`self.Ball`) (0.0 0.0 0.0) false "None"))

(fn `UserConstructionScript`)