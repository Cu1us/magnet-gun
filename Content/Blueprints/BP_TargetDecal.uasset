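; BP_TargetDecal is a decal indicator that marks a targeted position and shows whether it is valid.
; PointFromPos moves the decal to a world position and orients it along a given direction.
; It swaps between the target and invalid decal materials only when validity changes, tracked by ValidPosition.
; SetColor passes a color through to the decal component.
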(event `Set Color`
  (params (Color :type "LinearColor Structure"))
  (`DecalComponent.SetDecalColor` (`self.Decal`) Color))

(event `Point From Pos`
  (params (FromWS :type "Vector Structure") (`Point Dir` :type "Vector Structure") (`Valid Pos` :type Boolean))
  (bind _decal (`self.Decal`))
  (`SceneComponent.K2_SetWorldLocationAndRotation` (`self.Decal`) FromWS (`KismetMathLibrary.FindLookAtRotation` (`KismetMathLibrary.MakeVector` 0.0) `Point Dir`) false false)
  (if (!= (`self.Valid Position`) `Valid Pos`)
    (bind _output_get (set `self.Valid Position` `Valid Pos`))
    (if _output_get
      (`DecalComponent.SetDecalMaterial` _decal "/Game/Materials/M_TargetDecal.M_TargetDecal")
      (else
        (`DecalComponent.SetDecalMaterial` _decal "/Game/Materials/M_InvalidDecal.M_InvalidDecal")))))

(fn `UserConstructionScript`)