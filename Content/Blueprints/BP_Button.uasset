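; BP_Button is a physics-based button that detects when its movable top is pressed and released.
; Every tick, an acceleration-mode force along Z pushes ButtonTop at RiseSpeed, acting as the return spring.
; ButtonTrigger treats overlap begin and end with ButtonTop as press and release, currently only printing debug messages, including one for overlaps by other components.
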(event `self.ReceiveTick`
  (params (DeltaSeconds :type "Float (single-precision)"))
  (`PrimitiveComponent.AddForce` (`self.ButtonTop`) (`KismetMathLibrary.MakeVector` 0.0 0.0 (`self.RiseSpeed`)) "None" true))

(event `self.ButtonTrigger.OnComponentBeginOverlap`
  (params (OverlappedComponent :type "PrimitiveComponent Object Reference") (OtherActor :type "Actor Object Reference") (OtherComp :type "PrimitiveComponent Object Reference") (OtherBodyIndex :type Integer) (bFromSweep :type Boolean) (SweepResult :type "HitResult Structure (by ref)"))
  (if (== OtherComp (`self.ButtonTop`))
    (`KismetSystemLibrary.PrintString` "Pressed!")
    (else
      (`KismetSystemLibrary.PrintString` "Not pressed but overlap!"))))

(event `self.ButtonTrigger.OnComponentEndOverlap`
  (params (OverlappedComponent :type "PrimitiveComponent Object Reference") (OtherActor :type "Actor Object Reference") (OtherComp :type "PrimitiveComponent Object Reference") (OtherBodyIndex :type Integer))
  (if (== OtherComp (`self.ButtonTop`))
    (`KismetSystemLibrary.PrintString` "Unpressed!")))

(fn `UserConstructionScript`)