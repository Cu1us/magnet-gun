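; BP_Door is a double sliding door driven by an external ActivationSource, printing a warning at BeginPlay if none is valid.
; By default, the source's Activated and Deactivated events play and reverse the DoorSlide timeline.
; With DynamicOpen, Tick instead maps the source's activation value through DynamicOpenCurve.
; Both modes feed SetOpenAmount, which sweeps the two meshes in opposite directions along relative X, scaled by DoorOpenDistance.
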(event `self.ReceiveTick`
  (params (DeltaSeconds :type "Float (single-precision)"))
  (bind _activationsource (`self.ActivationSource`))
  (if (`self.Dynamic Open`)
    (`/Engine/EditorBlueprintResources/StandardMacros.IsValid` _activationsource
      (:`Is Valid`
        (bind (_isactive _activationvalue) (`/Game/Blueprints/BP_Activator.GetValue` _activationsource))
        (`self.SetOpenAmount` (`KismetMathLibrary.GetRuntimeFloatCurveValue` (`self.Dynamic Open Curve`) _activationvalue))))))

(event `self.ReceiveBeginPlay`
  (bind _activationsource (`self.ActivationSource`))
  (`/Engine/EditorBlueprintResources/StandardMacros.IsValid` _activationsource
    (:`Is Valid`
      (if (not (`self.Dynamic Open`))
        (add `/Game/Blueprints/BP_Activator.Activated` _activationsource (delegate `Open`))
        (add `/Game/Blueprints/BP_Activator.Deactivated` _activationsource (delegate `Close`))))
    (:`Is Not Valid`
      (`KismetSystemLibrary.PrintString` "Door was spawned without valid activation source!" true true (struct :`R` 1.0 :`G` 0.020499 :`A` 1.0) 5.0))))

(event `Open`
  (bind (_direction _opendistance) (`Timeline|DoorSlide` :!label _label)
    (:`Update`
      (`self.SetOpenAmount` _opendistance))))

(event `Close`
  (goto _label :!via `Reverse`))

(fn `SetOpenAmount`
  (params (`OpenAmount (0-1)` :type "Float (double-precision)"))
  (bind _returnvalue (`KismetMathLibrary.MakeVector` (* `OpenAmount (0-1)` (`self.DoorOpenDistance`))))
  (`|ExecutionSequence`
    (:`then_0`
      (`SceneComponent.K2_SetRelativeLocation` (`self.Door_DarkMetal1`) _returnvalue true false))
    (:`then_1`
      (`SceneComponent.K2_SetRelativeLocation` (`self.Door_DarkMetal`) (`KismetMathLibrary.NegateVector` _returnvalue) true false))))

(fn `UserConstructionScript`)