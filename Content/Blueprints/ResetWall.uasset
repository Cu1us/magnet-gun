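; ResetWall is a trigger actor that resets a set of balls when the first-person character passes through it in one direction.
; When the character stops overlapping, a dot product of the Plane's up vector and the direction to the capsule finds the exit side.
; An exit behind or level with the plane calls PerformReset, which has the player deselect each ball in BallsToReset, then resets that ball.
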(event `self.ReceiveActorEndOverlap`
  (params (OtherActor :type "Actor Object Reference"))
  (bind _plane (`self.Plane`))
  (bind _asbp_first_person_character (cast `/Game/Blueprints/BP_FirstPersonCharacter` OtherActor))
  (if (<= (`KismetMathLibrary.Dot_VectorVector` (`KismetMathLibrary.Normal` (- (`SceneComponent.K2_GetComponentLocation` (`Character.CapsuleComponent` _asbp_first_person_character)) (`SceneComponent.K2_GetComponentLocation` _plane))) (`SceneComponent.GetUpVector` _plane)) 0.0)
    (`self.Perform Reset`)))

(fn `Perform Reset`
  (locals (Player :type "/Game/Blueprints/BP_FirstPersonCharacter Object Reference"))
  (bind _returnvalue (`GameplayStatics.GetActorOfClass` "/Game/Blueprints/BP_FirstPersonCharacter.BP_FirstPersonCharacter_C"))
  (set `local.Player` _returnvalue)
  (for _array_element (`self.BallsToReset`)
    (`/Game/Blueprints/BP_FirstPersonCharacter.Deselect Ball` (`local.Player`) _array_element)
    (`/Game/Blueprints/BP_MagnetBall.Reset` _array_element)))

(fn `UserConstructionScript`)