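; BP_TriangleDoubleDoor is a two-panel sliding door whose openness is set by a normalized amount.
; SetOpenAmount stores the desired amount and slides DoorRight and DoorLeft in opposite directions along local X, scaled by DoorOpenDistance.
; Each move is swept, writing DoorsBlocked and updating ActualOpenAmount when unblocked, so the left panel's result overwrites the right's blocked flag.
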(fn `SetOpenAmount`
  (params (`OpenAmount (0-1)` :type "Float (double-precision)"))
  (bind _returnvalue (`KismetMathLibrary.MakeVector` (* `OpenAmount (0-1)` (`self.DoorOpenDistance`))))
  (set `self.Desired Open Amount` `OpenAmount (0-1)`)
  (`|ExecutionSequence`
    (:`then_0`
      (bind _sweephitresult (`SceneComponent.K2_SetRelativeLocation` (`self.DoorRight`) _returnvalue true false))
      (set `self.Doors Blocked` (`GameplayStatics.BreakHitResult` _sweephitresult)))
    (:`then_1`
      (bind _sweephitresult_2 (`SceneComponent.K2_SetRelativeLocation` (`self.DoorLeft`) (`KismetMathLibrary.NegateVector` _returnvalue) true false))
      (set `self.Doors Blocked` (`GameplayStatics.BreakHitResult` _sweephitresult_2))))
  (if (not (`self.Doors Blocked`))
    (set `self.Actual Open Amount` `OpenAmount (0-1)`)))

(fn `UserConstructionScript`)